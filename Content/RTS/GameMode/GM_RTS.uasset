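; RTS game mode that gives each joining player a random start camp and an RTS camera.
; On construction it gathers all PlayerStartCamp actors and prints their count.
; For each new player, it spawns a BP_RTSCamera at a random camp's camera location, possesses it and passes the camp to the controller.
; The camp then leaves the available pool, the player is recorded and the camp's tags are set.
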(event `self.ReceiveBeginPlay`)

(event `self.HandleStartingNewPlayer`
  (params (NewPlayer :type "PlayerController Object Reference"))
  (bind _outitem (`KismetArrayLibrary.Array_Random` (`self.List Player Start Camps`)))
  (`/Engine/EditorBlueprintResources/StandardMacros.IsValid` _outitem
    (:`Is Valid`
      (bind _output_get (set `self.Selected Start Camp` _outitem))
      (bind _returnvalue (`|SpawnActorFromClass` "/Game/RTS/BP_RTSCamera.BP_RTSCamera_C" (`SceneComponent.K2_GetComponentToWorld` (`/Game/RTS/PlayerStartCamp.CameraLocation` _output_get)) "Undefined" "MultiplyWithRoot" NewPlayer null))
      (`Controller.Possess` NewPlayer _returnvalue)
      (message `/Game/RTS/HUD/BP_SelectionInterface.SetupPlayerStart` NewPlayer (`self.Selected Start Camp`))
      (`KismetArrayLibrary.Array_RemoveItem` (`self.List Player Start Camps`) (`self.Selected Start Camp`))
      (`KismetArrayLibrary.Array_AddUnique` (`self.ListPlayer`) NewPlayer)
      (set `Actor.Tags` (`self.Tags_0`) (`self.Selected Start Camp`)))))

(fn `UserConstructionScript`
  (bind _outactors (`GameplayStatics.GetAllActorsOfClass` "/Game/RTS/PlayerStartCamp.PlayerStartCamp_C"))
  (bind _output_get (set `self.List Player Start Camps` _outactors))
  (`KismetSystemLibrary.PrintString` (`KismetStringLibrary.Conv_IntToString` (`KismetArrayLibrary.Array_Length` _output_get))))