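; RTS camera actor that becomes player 0's view target and pans when the mouse nears the screen edges.
; Each tick, four Move functions offset the root, ramping with cursor depth into the ScreenPourcentage border, without delta-time scaling.
; GetCameraSpeed scales pan speed with spring arm length.
; A debug-drawn trace along the camera's view then shifts the root vertically to keep ground distance near the arm length.
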(event `self.ReceiveBeginPlay`
  (`PlayerController.SetViewTargetWithBlend` (`GameplayStatics.GetPlayerController` 0) self 0.0 "VTBlend_Linear" 0.0 false))

(event `self.ReceiveTick`
  (params (DeltaSeconds :type "Float (single-precision)"))
  (`self.MoveLeft`)
  (`self.MoveRight`)
  (`self.MoveUp`)
  (`self.MoveDown`)
  (`self.AjustCameraPositionFromGround`))

(fn `AjustCameraPositionFromGround`
  (bind _defaultsceneroot (`self.DefaultSceneRoot`))
  (bind _camera (`self.Camera`))
  (bind _returnvalue (`SceneComponent.K2_GetComponentLocation` _camera))
  (bind (_outhit _returnvalue_2) (`KismetSystemLibrary.LineTraceSingle` :`Start` _returnvalue :`End` (+ _returnvalue (* (`SceneComponent.GetForwardVector` _camera) (* (`SpringArmComponent.TargetArmLength` (`self.SpringArm`)) 2.0))) :`TraceChannel` "TraceTypeQuery4" :`bTraceComplex` true :`DrawDebugType` "ForOneFrame"))
  (if _returnvalue_2
    (`SceneComponent.K2_AddRelativeLocation` _defaultsceneroot (* (`SceneComponent.GetUpVector` _defaultsceneroot) (`KismetMathLibrary.Conv_DoubleToVector` (- (`SpringArmComponent.TargetArmLength` (`self.SpringArm`)) (`.Distance` (`GameplayStatics.BreakHitResult` _outhit))))) false false)))

(fn `GetCameraSpeed`
  (params (ScaleFactor :type "Float (double-precision)"))
  (returns (ReturnValue :type "Float (double-precision)"))
  (return (* (+ (* (`KismetMathLibrary.NormalizeToRange` (`SpringArmComponent.TargetArmLength` (`self.SpringArm`)) (`self.DistanceCameraMinimale`) (`self.DistanceCameraMaximale`)) (`self.CameraMaxMoveSpeed`)) (`self.CameraMinMoveSpeed`)) ScaleFactor)))

(fn `MoveDown`
  (bind (_returnvalue_x _returnvalue_y) (`KismetMathLibrary.BreakVector2D` (`WidgetLayoutLibrary.GetViewportSize`)))
  (bind _returnvalue (`WidgetLayoutLibrary.GetMousePositionOnViewport`))
  (bind (_returnvalue_x_2 _returnvalue_y_2) (`KismetMathLibrary.BreakVector2D` (* _returnvalue (`WidgetLayoutLibrary.GetViewportScale`))))
  (`SceneComponent.K2_AddRelativeLocation` (`self.DefaultSceneRoot`) (* (* (* (`SceneComponent.GetForwardVector` (`self.DefaultSceneRoot`)) (`self.GetCameraSpeed` 1.0)) -1.0) (`KismetMathLibrary.FClamp` (`KismetMathLibrary.NormalizeToRange` _returnvalue_y_2 (* _returnvalue_y (- 1.0 (`self.ScreenPourcentage`))) _returnvalue_y))) false false))

(fn `MoveLeft`
  (bind _returnvalue_x (`KismetMathLibrary.BreakVector2D` (`WidgetLayoutLibrary.GetViewportSize`)))
  (bind _returnvalue (`WidgetLayoutLibrary.GetMousePositionOnViewport`))
  (bind _returnvalue_x_2 (`KismetMathLibrary.BreakVector2D` (* _returnvalue (`WidgetLayoutLibrary.GetViewportScale`))))
  (`SceneComponent.K2_AddRelativeLocation` (`self.DefaultSceneRoot`) (* (* (* (`SceneComponent.GetRightVector` (`self.DefaultSceneRoot`)) -1.0) (`self.GetCameraSpeed` 1.0)) (- 1.0 (`KismetMathLibrary.FClamp` (`KismetMathLibrary.NormalizeToRange` _returnvalue_x_2 0.0 (* _returnvalue_x (`self.ScreenPourcentage`)))))) false false))

(fn `MoveRight`
  (bind _returnvalue_x (`KismetMathLibrary.BreakVector2D` (`WidgetLayoutLibrary.GetViewportSize`)))
  (bind _returnvalue (`WidgetLayoutLibrary.GetMousePositionOnViewport`))
  (bind _returnvalue_x_2 (`KismetMathLibrary.BreakVector2D` (* _returnvalue (`WidgetLayoutLibrary.GetViewportScale`))))
  (`SceneComponent.K2_AddRelativeLocation` (`self.DefaultSceneRoot`) (* (* (`SceneComponent.GetRightVector` (`self.DefaultSceneRoot`)) (`self.GetCameraSpeed` 1.0)) (`KismetMathLibrary.FClamp` (`KismetMathLibrary.NormalizeToRange` _returnvalue_x_2 (* _returnvalue_x (- 1.0 (`self.ScreenPourcentage`))) _returnvalue_x))) false false))

(fn `MoveUp`
  (bind (_returnvalue_x _returnvalue_y) (`KismetMathLibrary.BreakVector2D` (`WidgetLayoutLibrary.GetViewportSize`)))
  (bind _returnvalue (`WidgetLayoutLibrary.GetMousePositionOnViewport`))
  (bind (_returnvalue_x_2 _returnvalue_y_2) (`KismetMathLibrary.BreakVector2D` (* _returnvalue (`WidgetLayoutLibrary.GetViewportScale`))))
  (`SceneComponent.K2_AddRelativeLocation` (`self.DefaultSceneRoot`) (* (* (`SceneComponent.GetForwardVector` (`self.DefaultSceneRoot`)) (`self.GetCameraSpeed` 1.0)) (- 1.0 (`KismetMathLibrary.FClamp` (`KismetMathLibrary.NormalizeToRange` _returnvalue_y_2 0.0 (* _returnvalue_y (`self.ScreenPourcentage`)))))) false false))

(fn `UserConstructionScript`)