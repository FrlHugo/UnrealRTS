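; RTS HUD that draws a drag-selection marquee and tracks the units inside it.
; External marquee press, hold and release events drive the rectangle, with direct events for single selection and clearing.
; While drawing, DrawHUD updates selection live through GetActorsInSelectionRectangle, messaging units to select or deselect and clearing any selected building.
; On release, it replaces PC_RTS's unit selection with its list.
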(event `self.ReceiveBeginPlay`
  (bind _aspc_rts (cast `/Game/RTS/PlayerController/PC_RTS` (`GameplayStatics.GetPlayerController` 0)))
  (set `self.As PC RTS` _aspc_rts))

(event `/Game/RTS/HUD/BP_SelectionInterface.Marquee Pressed`
  (bind (_locationx _locationy) (`PlayerController.GetMousePosition` (`GameplayStatics.GetPlayerController` 0)))
  ;[1 1 1] SELECTION START
  (set `self.isDrawing` true)
  (bind _output_get (set `self.StartMousePosition` (`KismetMathLibrary.MakeVector2D` _locationx _locationy)))
  (set `self.CurrentMousePosition` _output_get))

(event `/Game/RTS/HUD/BP_SelectionInterface.ClearSelectedUnits`
  (bind _listunitsselected (`self.ListUnitsSelected`))
  ;[1 1 1] Clear Selected Unit
  (for _array_element _listunitsselected
    (message `/Game/RTS/HUD/BP_SelectionInterface.DeselectThis` _array_element))
  (`KismetArrayLibrary.Array_Clear` _listunitsselected))

(event `/Game/RTS/HUD/BP_SelectionInterface.Marquee Held`
  (bind (_locationx _locationy) (`PlayerController.GetMousePosition` (`GameplayStatics.GetPlayerController` 0)))
  ;[1 1 1] Selection Held
  (set `self.CurrentMousePosition` (`KismetMathLibrary.MakeVector2D` _locationx _locationy)))

(event `/Game/RTS/HUD/BP_SelectionInterface.SelectSingleUnit`
  (params (Unit :type "Actor Object Reference"))
  ;[1 1 1] Select Single Unit
  (message `/Game/RTS/HUD/BP_SelectionInterface.SelectThis` Unit)
  (`KismetArrayLibrary.Array_AddUnique` (`self.ListUnitsSelected`) Unit))

(event `/Game/RTS/HUD/BP_SelectionInterface.Marquee Released`
  ;[1 1 1] Fin Selection
  (set `self.isDrawing` false)
  (`/Game/RTS/PlayerController/PC_RTS.ClearAllUnitsSelection` (`self.As PC RTS`))
  (for _array_element (`self.ListUnitsSelected`)
    (bind _asbp_character_units_base (cast `/Game/RTS/Units/BP_CharacterUnitsBase` _array_element))
    (`/Game/RTS/PlayerController/PC_RTS.AddUnitToSelection` (`self.As PC RTS`) _asbp_character_units_base)))

(event `self.ReceiveDrawHUD`
  (params (SizeX :type Integer) (SizeY :type Integer))
  (bind (_startmouseposition_x _startmouseposition_y) (`KismetMathLibrary.BreakVector2D` (`self.StartMousePosition`)))
  (bind (_currentmouseposition_x _currentmouseposition_y) (`KismetMathLibrary.BreakVector2D` (`self.CurrentMousePosition`)))
  ;[1 1 1] Rectangle de selection avec selection et déselection des unités
  ;;[1 1 1] Draw Rectangle
  (if (`self.isDrawing`)
    (`self.DrawRect` (struct :`R` 0.088542 :`G` 0.947314 :`B` 1.0 :`A` 0.5) _startmouseposition_x _startmouseposition_y (- _currentmouseposition_x _startmouseposition_x) (- _currentmouseposition_y _startmouseposition_y))
    ;;[1 1 1] Check For Actor Under The Rectangle
    (bind _output_get (set `self.ActorsInRectangle` (`self.GetActorsInSelectionRectangle` "/Game/RTS/Units/BP_CharacterUnitsBase.BP_CharacterUnitsBase_C" (`self.StartMousePosition`) (`self.CurrentMousePosition`) false)))
    (for _array_element _output_get
      ;;[0.3715 1 0.2292] Select Units under the rectangle
      (message `/Game/RTS/HUD/BP_SelectionInterface.SelectThis` _array_element)
      (`KismetArrayLibrary.Array_AddUnique` (`self.ListUnitsSelected`) _array_element)
      (message `/Game/RTS/HUD/BP_SelectionInterface.ClearSelectedBuilding` (`GameplayStatics.GetPlayerController` 0)))
    ;;[1 0.3902 0.3304] Deselect Units No Longuer under the rectangle
    (for _array_element_2 (`self.ListUnitsSelected`)
      (if (== (`KismetArrayLibrary.Array_Find` (`self.ActorsInRectangle`) _array_element_2) -1)
        (message `/Game/RTS/HUD/BP_SelectionInterface.DeselectThis` _array_element_2)
        (`KismetArrayLibrary.Array_RemoveItem` (`self.ListUnitsSelected`) _array_element_2)))))

(fn `GrabSelectedUnits`
  (returns (Units :type "Array of Actor Object Reference"))
  (return))

(fn `UserConstructionScript`)