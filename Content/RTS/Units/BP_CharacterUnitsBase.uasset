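; Base character Blueprint for RTS units, handling move commands and selection feedback.
; On BeginPlay it caches the RTS player controller and creates a selected-unit widget showing the unit's icon.
; Selection toggles a decal and adds that widget to the controller's selected-unit area or removes it, while highlighting swaps the decal material.
; Move commands run through AI MoveTo on the unit's AI controller.
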(event `self.UnitMoveCommand`
  (params (Location :type "Vector Structure"))
  ;[1 1 1] Unit Move
  (`AITask_MoveTo.AIMoveTo` (`AIBlueprintHelperLibrary.GetAIController` self) Location null))

(event `self.ReceiveBeginPlay`
  (bind _aspc_rts (cast `/Game/RTS/PlayerController/PC_RTS` (`GameplayStatics.GetPlayerController` 0)))
  (set `self.As PC RTS` _aspc_rts)
  ;[1 1 1] Set Unit WG
  (bind _returnvalue (`|CreateWidget` "/Game/RTS/UI/In_Game/WG_SelectedUnits.WG_SelectedUnits_C"))
  (bind _output_get (set `self.SelectedUnitWidget` _returnvalue))
  (set `/Game/RTS/UI/In_Game/WG_SelectedUnits.UnitReference` self _output_get)
  (`Image.SetBrushFromTexture` (`/Game/RTS/UI/In_Game/WG_SelectedUnits.Unit_Image` _returnvalue) (`self.2D_Icon`) false))

(event `IsSelected`
  (params (IsSelected :type Boolean))
  ;[1 1 1] Select Unit
  (`SceneComponent.SetVisibility` (`self.SelectionDecal`) IsSelected false))

(event `/Game/RTS/HUD/BP_SelectionInterface.HighlightUnit`
  ;[1 1 1] Select Unit
  (`DecalComponent.SetDecalMaterial` (`self.SelectionDecal`) "/Game/RTS/Units/MAT_HightightDecal.MAT_HightightDecal"))

(event `/Game/RTS/HUD/BP_SelectionInterface.UnHighlightUnit`
  ;[1 1 1] Select Unit
  (`DecalComponent.SetDecalMaterial` (`self.SelectionDecal`) "/Game/RTS/Units/MAT_unitsSelection2.MAT_unitsSelection2"))

(event `/Game/RTS/HUD/BP_SelectionInterface.SelectThis`
  ;[1 1 1] Select Unit
  (`SceneComponent.SetVisibility` (`self.SelectionDecal`) true false)
  (message `/Game/RTS/HUD/BP_SelectionInterface.AddUnitToSelectedUnitArea` (`GameplayStatics.GetPlayerController` 0) (`self.SelectedUnitWidget`)))

(event `/Game/RTS/HUD/BP_SelectionInterface.DeselectThis`
  ;[1 1 1] Select Unit
  (`SceneComponent.SetVisibility` (`self.SelectionDecal`) false false)
  (`Widget.RemoveFromParent` (`self.SelectedUnitWidget`)))

(fn `GrabSelectedUnits`
  (returns (Units :type "Array of Actor Object Reference"))
  (return))

(fn `UserConstructionScript`)