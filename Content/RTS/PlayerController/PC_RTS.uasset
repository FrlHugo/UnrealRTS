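; RTS player controller that handles unit and building selection, move orders and the player's starting camp.
; Left click selects a building under the cursor and forwards press, hold and release to the HUD for marquee selection.
; Right click writes TargetLocation into each selected unit's AI Blackboard and spawns a cursor effect.
; It also creates the selected-units widget, spawns the starting town hall and units at the camp, and prints debug output.
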(event `self.SetupPlayerStart`
  (params (PlayerStartCamp :type "/Game/RTS/PlayerStartCamp Object Reference"))
  (`self.LoadStartBuilding&Units` PlayerStartCamp))

(event `self.ClearSelectedBuilding`
  (bind _selectbuilding (`self.SelectBuilding`))
  ;[1 1 1] Clear Selected Building
  (`/Engine/EditorBlueprintResources/StandardMacros.IsValid` _selectbuilding
    (:`Is Valid`
      (message `/Game/RTS/HUD/BP_SelectionInterface.DeselectThis` _selectbuilding)
      (set `self.SelectBuilding` null))))

(event `self.AddUnitToSelectedUnitArea`
  (params (WG_SelectedUnit :type "UserWidget Object Reference"))
  (bind _wg_selectedunitarea (`self.WG_SelectedUnitArea`))
  (`KismetSystemLibrary.PrintString` (`KismetSystemLibrary.GetDisplayName` _wg_selectedunitarea) true true (struct :`R` 1.0 :`G` 0.703581 :`A` 1.0) 20.0 "1None")
  (`KismetSystemLibrary.PrintString` (`KismetSystemLibrary.GetDisplayName` WG_SelectedUnit) true true (struct :`R` 1.0 :`B` 0.237192 :`A` 1.0) 202.0 "2")
  (`HorizontalBox.AddChildToHorizontalBox` (`/Game/RTS/UI/In_Game/WG_SelectedUnitsArea.HB_UnitBox` _wg_selectedunitarea) WG_SelectedUnit))

(event `self.ReceiveBeginPlay`
  (if (`self.IsLocalPlayerController`)
    _
    (else
      _))
  (`WidgetBlueprintLibrary.SetInputMode_GameAndUIEx` self null "LockAlways" false)
  (bind _returnvalue (`|CreateWidget` "/Game/RTS/UI/In_Game/WG_SelectedUnitsArea.WG_SelectedUnitsArea_C"))
  (bind _output_get (set `self.WG_SelectedUnitArea` _returnvalue))
  (`UserWidget.AddToViewport` _output_get 0))

(event `Key|Z`
  (params (Key :type "Key Structure"))
  (:`Pressed`
    (`self.ClearAllUnitsSelection`)))

(event `self.ReceiveTick`
  (params (DeltaSeconds :type "Float (single-precision)"))
  (`KismetSystemLibrary.PrintString` (`KismetStringLibrary.Conv_IntToString` (`KismetArrayLibrary.Array_Length` (`self.ListUnitSelection`))) true true (struct :`G` 0.66 :`B` 1.0 :`A` 1.0) 25.0)
  (if (`self.isLeftButtonPressed`)
    (message `/Game/RTS/HUD/BP_SelectionInterface.Marquee Held` (`self.GetHUD`))))

(event `Key|LeftMouseButton`
  (params (Key :type "Key Structure"))
  (bind _returnvalue (`self.GetHUD`))
  (:`Pressed`
    (set `self.isLeftButtonPressed` true)
    (`self.HandleBuildingClick`)
    (message `/Game/RTS/HUD/BP_SelectionInterface.Marquee Pressed` _returnvalue))
  (:`Released`
    (set `self.isLeftButtonPressed` false)
    (message `/Game/RTS/HUD/BP_SelectionInterface.Marquee Released` _returnvalue)))

(event `Key|Escape`
  (params (Key :type "Key Structure"))
  (:`Pressed`
    (`KismetSystemLibrary.QuitGame` null "Quit")))

(event `Key|RightMouseButton`
  (params (Key :type "Key Structure"))
  (bind _hitresult (`self.GetHitResultUnderCursorByChannel` "TraceTypeQuery1"))
  ;[1 1 1] Moving Units
  (:`Pressed`
    (if (`.ReturnValue` (`self.GetHitResultUnderCursorByChannel` "TraceTypeQuery4"))
      (for _array_element (`self.ListUnitSelection`)
        (`BlackboardComponent.SetValueAsVector` (`AIBlueprintHelperLibrary.GetBlackboard` _array_element) "TargetLocation" (`.Location` (`GameplayStatics.BreakHitResult` _hitresult)))
        (`NiagaraFunctionLibrary.SpawnSystemAtLocation` "/Game/RTS/Cursor/FX_Cursor.FX_Cursor" (`.Location` (`GameplayStatics.BreakHitResult` _hitresult)) (struct) (4.0 4.0 4.0))))))

(fn `AddUnitToSelection`
  (params (UnitBase :type "/Game/RTS/Units/BP_CharacterUnitsBase Object Reference"))
  (`KismetArrayLibrary.Array_AddUnique` (`self.ListUnitSelection`) UnitBase)
  (`/Game/RTS/Units/BP_CharacterUnitsBase.IsSelected` UnitBase true))

(fn `ClearAllUnitsSelection`
  (for _array_element (`self.ListUnitSelection`)
    (`/Game/RTS/Units/BP_CharacterUnitsBase.IsSelected` _array_element false))
  (`KismetArrayLibrary.Array_Clear` (`self.ListUnitSelection`)))

(fn `GrabSelectedUnits`
  (returns (Units :type "Array of Actor Object Reference"))
  (return))

(fn `NewFunction`)

(fn `RemoveUnitFromSelection`
  (params (Unit :type "/Game/RTS/Units/BP_CharacterUnitsBase Object Reference"))
  (`KismetArrayLibrary.Array_RemoveItem` (`self.ListUnitSelection`) Unit)
  (`/Game/RTS/Units/BP_CharacterUnitsBase.IsSelected` Unit false))

(fn `UserConstructionScript`)