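; RTS HUD that draws a translucent drag rectangle for marquee unit selection.
; Marquee press, hold and release events track mouse corners, while DrawHUD queries actors inside the rectangle each frame, sending select and deselect messages to keep the unit list current.
; Release passes listed units to AsPCRTS, though BeginPlay sets that reference to None.
; StartSelection and StopSelection are empty, and an older marquee implementation remains disconnected.
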(event `self.ReceiveBeginPlay`
  (bind _aspc_rts (cast `` (`GameplayStatics.GetPlayerController` 0)))
  (set `self.As PC RTS` null _aspc_rts))

(event `self.StartSelection`)

(event `self.StopSelection`)

(event `self.Marquee Pressed`
  (bind (_locationx _locationy) (`PlayerController.GetMousePosition` (`GameplayStatics.GetPlayerController` 0)))
  ;[1 1 1] SELECTION START
  (set `self.isDrawing` true)
  (bind _output_get (set `self.StartMousePosition` (`KismetMathLibrary.MakeVector2D` _locationx _locationy)))
  (set `self.CurrentMousePosition` _output_get))

(event `self.Marquee Held`
  (bind (_locationx _locationy) (`PlayerController.GetMousePosition` (`GameplayStatics.GetPlayerController` 0)))
  ;[1 1 1] Selection Held
  (set `self.CurrentMousePosition` (`KismetMathLibrary.MakeVector2D` _locationx _locationy)))

(event `self.Marquee Released`
  ;[1 1 1] Fin Selection
  (set `self.isDrawing` false)
  (for _array_element (`self.ListUnitsSelected`)
    (bind _asbp_character_units_base (cast `` _array_element))
    (`self.AddUnitToSelection` (`.As PC RTS` (`self.As PC RTS`)) _asbp_character_units_base)))

(event `self.ReceiveDrawHUD`
  (params (SizeX :type Integer) (SizeY :type Integer))
  (bind (_startmouseposition_x _startmouseposition_y) (`KismetMathLibrary.BreakVector2D` (`self.StartMousePosition`)))
  (bind (_currentmouseposition_x _currentmouseposition_y) (`KismetMathLibrary.BreakVector2D` (`self.CurrentMousePosition`)))
  ;[1 1 1] Rectangle de selection avec selection et déselection des unités
  (if (`self.isDrawing`)
    (`self.DrawRect` (struct :`R` 0.088542 :`G` 0.947314 :`B` 1.0 :`A` 0.5) _startmouseposition_x _startmouseposition_y (- _currentmouseposition_x _startmouseposition_x) (- _currentmouseposition_y _startmouseposition_y))
    (bind _output_get (set `self.ActorsInRectangle` (`self.GetActorsInSelectionRectangle` null (`self.StartMousePosition`) (`self.CurrentMousePosition`) false)))
    (for _array_element _output_get
      (message `/Game/HUD/BP_RTSHUD.Select Unit` _array_element)
      (`KismetArrayLibrary.Array_AddUnique` (`self.ListUnitsSelected`) _array_element))
    (for _array_element_2 (`self.ListUnitsSelected`)
      (if (== (`KismetArrayLibrary.Array_Find` (`self.ActorsInRectangle`) _array_element_2) -1)
        (message `/Game/HUD/BP_RTSHUD.Deselect Unit` _array_element_2)
        (`KismetArrayLibrary.Array_RemoveItem` (`self.ListUnitsSelected`) _array_element_2)))))

(fn `UserConstructionScript`)