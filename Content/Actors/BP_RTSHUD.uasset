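; BP_RTSHUD is a HUD that draws a drag-selection box for RTS-style mouse selection.
; StartSelection stores the mouse position, scaled by viewport scale, as the anchor corner and enables drawing, while StopSelection disables it.
; While drawing is active, DrawHUD samples the current scaled mouse position each frame and renders a translucent cyan rectangle from the anchor to it.
; It only draws the box and does not gather selected actors.
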(event `/Game/UI/BP_SelectionInterface.StartSelection`
  (bind _returnvalue (`WidgetLayoutLibrary.GetMousePositionOnViewport`))
  (set `self.PointA` (* _returnvalue (`WidgetLayoutLibrary.GetViewportScale`)))
  (set `self.isDrawing` true))

(event `/Game/UI/BP_SelectionInterface.StopSelection`
  (set `self.isDrawing` false))

(event `self.ReceiveDrawHUD`
  (params (SizeX :type Integer) (SizeY :type Integer))
  (bind (_pointa_x _pointa_y) (`KismetMathLibrary.BreakVector2D` (`self.PointA`)))
  (bind (_pointb_x _pointb_y) (`KismetMathLibrary.BreakVector2D` (`self.PointB`)))
  (if (`self.isDrawing`)
    (bind _returnvalue (`WidgetLayoutLibrary.GetMousePositionOnViewport`))
    (set `self.PointB` (* _returnvalue (`WidgetLayoutLibrary.GetViewportScale`)))
    (`self.DrawRect` (struct :`R` 0.088542 :`G` 0.947314 :`B` 1.0 :`A` 0.5) _pointa_x _pointa_y (- _pointb_x _pointa_x) (- _pointb_y _pointa_y))))

(fn `UserConstructionScript`)