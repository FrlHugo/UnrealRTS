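; PC_RTS is the RTS player controller, handling camera zoom and unit selection input.
; On BeginPlay it locks the mouse in Game and UI mode, then caches the BP_Camera view target and sets its distance limits.
; Mouse wheel input adjusts a clamped zoom factor that drives the camera's spring arm length.
; Left-click press and release signal selection to the HUD, while add/remove functions maintain the selected unit list and flag each unit.
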(event `self.ReceiveBeginPlay`
  (`WidgetBlueprintLibrary.SetInputMode_GameAndUIEx` self null "LockAlways" false)
  (bind _asbp_camera (cast `/Game/Actors/BP_Camera` (`self.GetViewTarget`)))
  (bind _output_get (set `self.As RTSCamera` _asbp_camera))
  (set `/Game/Actors/BP_Camera.DistanceCameraMinimale` (`self.DistanceCameraMinimale`) _output_get)
  (set `/Game/Actors/BP_Camera.DistanceCameraMaximale` (+ (* (`self.ZoomMax`) (`self.MultiplicateurDistanceCamera`)) (`self.DistanceCameraMinimale`)) _output_get))

(event `InputAxisKey|MouseWheelAxis`
  (params (AxisValue :type "Float (single-precision)"))
  (bind _output_get (set `self.ZoomFactor` (`KismetMathLibrary.FClamp` (+ (`self.ZoomFactor`) AxisValue) (`self.ZoomMin`) (`self.ZoomMax`))))
  (set `SpringArmComponent.TargetArmLength` (+ (* _output_get (`self.MultiplicateurDistanceCamera`)) (`self.DistanceCameraMinimale`)) (`/Game/Actors/BP_Camera.SpringArm` (`self.As RTSCamera`))))

(event `Key|LeftMouseButton`
  (params (Key :type "Key Structure"))
  (bind _returnvalue (`self.GetHUD`))
  (:`Pressed`
    (message `/Game/UI/BP_SelectionInterface.StartSelection` _returnvalue))
  (:`Released`
    (message `/Game/UI/BP_SelectionInterface.StopSelection` _returnvalue)))

(fn `AddUnitToSelection`
  (params (UnitBase :type "/Game/Units/BP_CharacterUnits Object Reference"))
  (`KismetArrayLibrary.Array_AddUnique` (`self.ListUnitSelection`) UnitBase)
  (`/Game/Units/BP_CharacterUnits.IsSelected` UnitBase true))

(fn `RemoveUnitFromSelection`
  (params (Unit :type "/Game/Units/BP_CharacterUnits Object Reference"))
  (`KismetArrayLibrary.Array_RemoveItem` (`self.ListUnitSelection`) Unit)
  (`/Game/Units/BP_CharacterUnits.IsSelected` Unit false))

(fn `UserConstructionScript`)