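; Base character for RTS units that can be click-selected and ordered to move.
; A left click asks a cast object, likely the RTS player controller, to add or remove the unit from its selection, using decal visibility as the selected state.
; SelectUnit and DeselectUnit show or hide that decal, and UnitMoveCommand sends the AI controller to a location through AIMoveTo.
; The IsSelected event is an empty stub.
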(event `self.ReceiveBeginPlay`
  (bind _aspc_rts (cast `` (`GameplayStatics.GetPlayerController` 0)))
  (set `self.As PC RTS` null _aspc_rts))

(event `self.ReceiveActorOnClicked`
  (params (ButtonPressed :type "Key Structure"))
  (if (== ButtonPressed "LeftMouseButton")
    (bind _aspc_rts (cast `` _))
    (if (`SceneComponent.IsVisible` (`self.Decal`))
      (`self.RemoveUnitFromSelection` _aspc_rts self)
      (else
        (`self.AddUnitToSelection` _aspc_rts self)))))

(event `IsSelected`
  (params (IsSelected :type Boolean)))

(event `self.Select Unit`
  (`SceneComponent.SetVisibility` (`self.Decal`) true false))

(event `self.Deselect Unit`
  (`SceneComponent.SetVisibility` (`self.Decal`) false false))

(event `self.UnitMoveCommand`
  (params (Location :type "Vector Structure"))
  (`AITask_MoveTo.AIMoveTo` (`AIBlueprintHelperLibrary.GetAIController` self) Location null))

(fn `UserConstructionScript`)