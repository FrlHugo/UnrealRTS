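; BP_CharacterUnits is a selectable RTS unit character that the player toggles in and out of the current selection.
; A left click casts the player controller to PC_RTS and adds or removes the unit, using the selection decal's visibility as the selected state.
; The IsSelected event shows or hides that decal to reflect selection.
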(event `self.ReceiveActorOnClicked`
  (params (ButtonPressed :type "Key Structure"))
  (if (== ButtonPressed "LeftMouseButton")
    (bind _aspc_rts (cast `/Game/PlayerController/PC_RTS` (`GameplayStatics.GetPlayerController` 0)))
    (if (`SceneComponent.IsVisible` (`self.Decal`))
      (`/Game/PlayerController/PC_RTS.RemoveUnitFromSelection` _aspc_rts self)
      (else
        (`/Game/PlayerController/PC_RTS.AddUnitToSelection` _aspc_rts self)))))

(event `IsSelected`
  (params (IsSelected :type Boolean))
  (`SceneComponent.SetVisibility` (`self.Decal`) IsSelected false))

(fn `UserConstructionScript`)